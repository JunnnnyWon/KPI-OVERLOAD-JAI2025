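; Projectile actor that damages and knocks back enemies and destroys enemy projectiles.
; Tick moves it by its velocity with a swept offset, and hitting anything but the player pawn stops, hides and disables its collision without destroying it.
; Hit casts separately to Tank, Manager, base enemy and enemy projectile classes.
; Enemies are launched along the bullet's forward vector, lose fixed health and are destroyed only at exactly zero.
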(event `self.ReceiveTick`
  (params (DeltaSeconds :type "Float (single-precision)"))
  (`self.K2_AddActorWorldOffset` (* DeltaSeconds (`self.BulletVelocity`)) true true))

(event `self.ReceiveHit`
  (params (MyComp :type "PrimitiveComponent Object Reference") (Other :type "Actor Object Reference") (OtherComp :type "PrimitiveComponent Object Reference") (bSelfMoved :type Boolean) (HitLocation :type "Vector Structure") (HitNormal :type "Vector Structure") (NormalImpulse :type "Vector Structure") (Hit :type "HitResult Structure (by ref)"))
  (`|ExecutionSequence`
    (:`then_0`
      (if (!= Other (`GameplayStatics.GetPlayerPawn` 0))
        (set `self.BulletVelocity` (0.0 0.0 0.0))
        (`self.SetActorHiddenInGame` true)
        (`self.SetActorEnableCollision` false)))
    (:`then_1`
      (bind _asbp_enemy_tank (cast `/Game/1_KPI_Character/BP_Enemy_Tank` Other))
      (`Character.LaunchCharacter` _asbp_enemy_tank (* (`self.GetActorForwardVector`) (1000.0 1000.0 0.0)) true true)
      (bind _output_get (set `/Game/1_KPI_Character/BP_Enemy_Tank.Health` (- (`/Game/1_KPI_Character/BP_Enemy_Tank.Health` _asbp_enemy_tank) 25.0) _asbp_enemy_tank))
      (if (== _output_get 0.0)
        (`self.K2_DestroyActor` _asbp_enemy_tank)))
    (:`then_2`
      (bind _asbp_enemy_projectile (cast `/Game/1_KPI_Character/BP_EnemyProjectile` Other))
      (`self.K2_DestroyActor` _asbp_enemy_projectile))
    (:`then_3`
      (bind _asbp_enemy_the_manager (cast `/Game/1_KPI_Character/BP_Enemy_The_Manager` Other))
      (`Character.LaunchCharacter` _asbp_enemy_the_manager (* (`self.GetActorForwardVector`) (1000.0 1000.0 0.0)) true true)
      (bind _output_get_2 (set `/Game/1_KPI_Character/BP_Enemy_The_Manager.Health` (- (`/Game/1_KPI_Character/BP_Enemy_The_Manager.Health` _asbp_enemy_the_manager) 25.0) _asbp_enemy_the_manager))
      (if (== _output_get_2 0.0)
        (`self.K2_DestroyActor` _asbp_enemy_the_manager)))
    (:`then_4`
      (bind _asbp_enemy_base (cast `/Game/1_KPI_Character/BP_EnemyBase` Other))
      (`Character.LaunchCharacter` _asbp_enemy_base (* (`self.GetActorForwardVector`) (1000.0 1000.0 0.0)) true true)
      (bind _output_get_3 (set `/Game/1_KPI_Character/BP_EnemyBase.health` (- (`/Game/1_KPI_Character/BP_EnemyBase.health` _asbp_enemy_base) 25.0) _asbp_enemy_base))
      (if (== _output_get_3 0.0)
        (`self.K2_DestroyActor` _asbp_enemy_base)))))

(fn `UserConstructionScript`)