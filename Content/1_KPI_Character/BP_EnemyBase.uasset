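; BP_EnemyBase is a base enemy that chases the player.
; Each tick it calls EnemyMove, which adds movement input along the normalized direction from itself to player pawn 0, with no pathfinding.
; Hitting a BP_PlayerPawn only prints a debug message as a placeholder for damage logic.
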(event `self.ReceiveBeginPlay`)

(event `self.ReceiveTick`
  (params (DeltaSeconds :type "Float (single-precision)"))
  (`self.EnemyMove`))

(event `EnemyMove`
  (`self.AddMovementInput` (`KismetMathLibrary.Normal` (- (`self.K2_GetActorLocation` (`GameplayStatics.GetPlayerPawn` 0)) (`self.K2_GetActorLocation`)))))

(event `self.ReceiveHit`
  (params (MyComp :type "PrimitiveComponent Object Reference") (Other :type "Actor Object Reference") (OtherComp :type "PrimitiveComponent Object Reference") (bSelfMoved :type Boolean) (HitLocation :type "Vector Structure") (HitNormal :type "Vector Structure") (NormalImpulse :type "Vector Structure") (Hit :type "HitResult Structure (by ref)"))
  (cast `/Game/1_KPI_Character/BP_PlayerPawn` Other)
  (`KismetSystemLibrary.PrintString` "Player Hit ! Damage to player Logic !"))

(fn `UserConstructionScript`)