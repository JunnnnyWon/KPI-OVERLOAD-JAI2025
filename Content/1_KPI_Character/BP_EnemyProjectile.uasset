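; BP_EnemyProjectile is an enemy projectile that homes in on the player and deals damage on contact.
; On BeginPlay it sets the player pawn's root component as the homing target of its ProjectileMovement component.
; Overlapping BP_PlayerPawn subtracts a fixed amount from PlayerHealth, destroys the projectile and plays a world damage camera shake centered on the player.
; The Hit event is empty, so only overlaps with the player have an effect.
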(event `self.ReceiveBeginPlay`
  (set `ProjectileMovementComponent.HomingTargetComponent` (`Actor.RootComponent` (`GameplayStatics.GetPlayerPawn` 0)) (`self.ProjectileMovement`)))

(event `self.ReceiveActorBeginOverlap`
  (params (OtherActor :type "Actor Object Reference"))
  (bind _asbp_player_pawn (cast `/Game/1_KPI_Character/BP_PlayerPawn` OtherActor))
  (set `/Game/1_KPI_Character/BP_PlayerPawn.PlayerHealth` (- (`/Game/1_KPI_Character/BP_PlayerPawn.PlayerHealth` _asbp_player_pawn) 10.0) _asbp_player_pawn)
  (`self.K2_DestroyActor`)
  (`GameplayStatics.PlayWorldCameraShake` "/Game/1_KPI_Character/CS_Damage.CS_Damage_C" (`self.K2_GetActorLocation` _asbp_player_pawn) 5000.0 10000.0))

(event `self.ReceiveHit`
  (params (MyComp :type "PrimitiveComponent Object Reference") (Other :type "Actor Object Reference") (OtherComp :type "PrimitiveComponent Object Reference") (bSelfMoved :type Boolean) (HitLocation :type "Vector Structure") (HitNormal :type "Vector Structure") (NormalImpulse :type "Vector Structure") (Hit :type "HitResult Structure (by ref)")))

(fn `UserConstructionScript`)