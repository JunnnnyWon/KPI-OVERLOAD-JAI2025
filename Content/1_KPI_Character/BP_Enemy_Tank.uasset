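; BP_Enemy_Tank is an enemy pawn that chases the player while emitting radial force impulses.
; Every Tick fires the RadialForce component's impulse, then calls the EnemyMove event.
; EnemyMove adds movement input along the normalized direction toward player pawn 0, steering straight at it without pathfinding.
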(event `EnemyMove`
  (`self.AddMovementInput` (`KismetMathLibrary.Normal` (- (`self.K2_GetActorLocation` (`GameplayStatics.GetPlayerPawn` 0)) (`self.K2_GetActorLocation`)))))

(event `self.ReceiveTick`
  (params (DeltaSeconds :type "Float (single-precision)"))
  (`|ExecutionSequence`
    (:`then_0`
      (`RadialForceComponent.FireImpulse` (`self.RadialForce`)))
    (:`then_1`
      (`self.EnemyMove`))))

(fn `UserConstructionScript`)