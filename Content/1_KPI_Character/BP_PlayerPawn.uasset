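; BP_PlayerPawn is a top-down player pawn that aims at the mouse cursor and moves by firing recoil.
; Tick turns it toward the cursor's hit point and eases the spring arm offset that way.
; Left click starts looping fire that impulses the sphere backward, shakes the camera and launches bullets from a pool pre-spawned at BeginPlay.
; Right click stops firing and switches the sphere to its stopping damping.
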(event `self.ReceiveTick`
  (params (DeltaSeconds :type "Float (single-precision)"))
  (bind _returnvalue (`self.K2_GetActorLocation`))
  (bind _springarm (`self.SpringArm`))
  (bind _hitresult (`PlayerController.GetHitResultUnderCursorByChannel` (`GameplayStatics.GetPlayerController` 0) "TraceTypeQuery1" true))
  (`self.K2_SetActorRotation` (`KismetMathLibrary.FindLookAtRotation` _returnvalue (`KismetMathLibrary.MakeVector` (.x (`.Location` (`GameplayStatics.BreakHitResult` _hitresult))) (.y (`.Location` (`GameplayStatics.BreakHitResult` _hitresult))) (.z _returnvalue))))
  (set `SpringArmComponent.SocketOffset` (`KismetMathLibrary.VInterpTo` (`SpringArmComponent.SocketOffset` _springarm) (* (- (`.Location` (`GameplayStatics.BreakHitResult` _hitresult)) _returnvalue) 0.1)) _springarm))

(event `Key|RightMouseButton`
  (params (Key :type "Key Structure"))
  (:`Pressed`
    (`KismetSystemLibrary.K2_ClearAndInvalidateTimerHandle` (`self.TimerHandle`))
    (`PrimitiveComponent.SetLinearDamping` (`self.Sphere`) (`self.LinearDamping_Stop`))))

(event `Key|LeftMouseButton`
  (params (Key :type "Key Structure"))
  (:`Pressed`
    (bind _returnvalue (`KismetSystemLibrary.K2_SetTimerDelegate` (delegate `ExecutreFire`) (/ 1.0 (`self.FireRate`)) true))
    (set `self.TimerHandle` _returnvalue)))

(event `ExecutreFire`
  (`PrimitiveComponent.SetLinearDamping` (`self.Sphere`) (`self.LinearDamping_Move`))
  (bind _output_get (set `self.RecoilDir` (* (`self.GetActorForwardVector`) (-1.0 -1.0 0.0))))
  (set `self.ImpulseVec` (* _output_get (`self.Recoil Force`)))
  (`PrimitiveComponent.AddImpulse` (`self.Sphere`) (`self.ImpulseVec`) "None" true)
  (bind _foundbullet (`self.GetBulletFromPool`))
  (`self.SetActorTickEnabled` _foundbullet true)
  (`self.K2_SetActorLocationAndRotation` _foundbullet (`SceneComponent.K2_GetComponentLocation` (`self.MuzzleArrow`)) (`self.K2_GetActorRotation`) false true)
  (set `/Game/1_KPI_Character/BP_Bullet.BulletVelocity` (* (`self.GetActorForwardVector` (`GameplayStatics.GetPlayerPawn` 0)) 3000.0) _foundbullet)
  (`self.SetActorHiddenInGame` _foundbullet false)
  (`self.SetActorEnableCollision` _foundbullet true)
  (`GameplayStatics.PlayWorldCameraShake` "/Game/1_KPI_Character/CS_Shooting.CS_Shooting_C" (`self.K2_GetActorLocation`) 5000.0 10000.0))

(event `self.ReceiveBeginPlay`
  (set `PlayerController.bShowMouseCursor` true (`GameplayStatics.GetPlayerController` 0))
  (for _ (range 21)
    (bind _returnvalue (`|SpawnActorFromClass` "/Game/1_KPI_Character/BP_Bullet.BP_Bullet_C" (`KismetMathLibrary.MakeTransform` (0.0 0.0 0.0)) "Undefined" "MultiplyWithRoot" null null))
    (`self.SetActorHiddenInGame` _returnvalue true)
    (`self.SetActorEnableCollision` _returnvalue false)
    (`KismetArrayLibrary.Array_Add` (`self.BulletPool`) _returnvalue)))

(fn `GetBulletFromPool`
  (returns (FoundBullet :type "/Game/1_KPI_Character/BP_Bullet Object Reference"))
  (for _array_element (`self.BulletPool`)
    (if (`Actor.bHidden` _array_element)
      (return _array_element))))

(fn `UserConstructionScript`)